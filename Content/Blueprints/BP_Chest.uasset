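; Chest that opens once when interacted with, provided the player's BP_Player character holds at least two keys.
; Interact calls TryOpenChest, which checks the key count without decrementing it and uses a DoOnce to block repeat openings.
; Three chained timelines animate the sequence: both key meshes appear and slide in, their pivots turn, then the keys hide and the lid pivot swings open.
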(event `/Game/Lesson/InheritanceExample/BPI_Interaction.Interact`
  (`self.TryOpenChest`))

(event `TryOpenChest`
  (bind _keymesh_left (`self.KeyMesh_Left`))
  (bind _keymesh_right (`self.KeyMesh_Right`))
  (bind _asbp_player (cast `/Game/Lesson/Blueprints/BP_Player` (`GameplayStatics.GetPlayerCharacter` 0)))
  (if (>= (`/Game/Lesson/Blueprints/BP_Player.NbKeys` _asbp_player) 2)
    (`/Engine/EditorBlueprintResources/StandardMacros.DoOnce` false
      (:`Completed`
        (`SceneComponent.SetVisibility` (`self.KeyMesh_Right`) true false)
        (`SceneComponent.SetVisibility` (`self.KeyMesh_Left`) true false)
        (bind (_direction _insert) (`Timeline|TL_InsertKey` :!via `PlayFromStart`)
          (:`Update`
            (bind _returnvalue (`KismetMathLibrary.Lerp` 28.0 8.0 _insert))
            (`SceneComponent.K2_SetRelativeLocation` _keymesh_right (`KismetMathLibrary.MakeVector` 0.0 _returnvalue) false false)
            (`SceneComponent.K2_SetRelativeLocation` _keymesh_left (`KismetMathLibrary.MakeVector` 0.0 _returnvalue) false false))
          (:`Finished`
            (bind (_direction_2 _turn) (`Timeline|TL_TurnKey` :!via `PlayFromStart`)
              (:`Update`
                (bind _returnvalue_2 (* _turn 30.0))
                (`SceneComponent.K2_SetRelativeRotation` (`self.KeyPivot_Left`) (`KismetMathLibrary.MakeRotator` 0.0 _returnvalue_2) false false)
                (`SceneComponent.K2_SetRelativeRotation` (`self.KeyPivot_Right`) (`KismetMathLibrary.MakeRotator` 0.0 _returnvalue_2) false false))
              (:`Finished`
                (`SceneComponent.SetVisibility` _keymesh_right false false)
                (`SceneComponent.SetVisibility` _keymesh_left false false)
                (bind (_direction_3 _open) (`Timeline|Timeline` :!via `PlayFromStart`)
                  (:`Update`
                    (`SceneComponent.K2_SetRelativeRotation` (`self.LidPivot`) (`KismetMathLibrary.MakeRotator` (* _open -75.0)) false false)))))))))))

(fn `UserConstructionScript`)