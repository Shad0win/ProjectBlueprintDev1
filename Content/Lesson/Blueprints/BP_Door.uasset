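; BP_Door is a double door that swings open when its Interact event fires.
; Interact sets the Enzo timeline's play rate from TimeOpenDoor, so the opening duration is tunable, then plays it.
; Each timeline update scales DoorAngle by the OpenDoor track to yaw the two door meshes in opposite directions.
; When the timeline finishes it prints a debug message; the graph contains no closing logic.
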(event `/Game/Lesson/InheritanceExample/BPI_Interaction.Interact`
  (`TimelineComponent.SetPlayRate` (`self.Enzo`) (/ 1.0 (`self.TimeOpenDoor`)))
  (bind (_direction _opendoor) (`Timeline|Enzo`)
    (:`Update`
      (bind _returnvalue (* _opendoor (`self.DoorAngle`)))
      (`SceneComponent.K2_SetRelativeRotation` (`self.Door_3_StaticMeshComponent0`) (`KismetMathLibrary.MakeRotator` 0.0 0.0 (* _returnvalue -1.0)) false false)
      (`SceneComponent.K2_SetRelativeRotation` (`self.Door_4_StaticMeshComponent0`) (`KismetMathLibrary.MakeRotator` 0.0 0.0 _returnvalue) false false))
    (:`Finished`
      (`KismetSystemLibrary.PrintString` "DOOR IS OPEN"))))

(fn `UserConstructionScript`)